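; Game mode Blueprint that handles checkpoint respawning for the player character.
; On BeginPlay it caches the PlayerCharacterTwo player and binds to its health component's health-ended event.
; EventDeath teleports the player to the stored save point's transform and restores full health, provided a save point is valid.
; SetSavePoint stores the new point and prints a message unless it is flagged as the first point.
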(event `self.ReceiveBeginPlay`
  (bind _asplayer_character_two (cast `/Game/Actors/Characters/Player/PlayerCharacterTwo` (`GameplayStatics.GetPlayerCharacter` 0)))
  (bind _output_get (set `self.PlayerCharacter` _asplayer_character_two))
  (add `HealthComponent.OnHealthEnded` (`/Game/Actors/Characters/Player/PlayerCharacter.HealthComponentPlayer` _output_get) (`|CreateDelegate` :!event `EventDeath`)))

(fn `EventDeath`
  (params (Value :type "Float (double-precision)") (Instigator :type "Actor Object Reference"))
  (bind _playercharacter (`self.PlayerCharacter`))
  (bind _savepoint (`self.SavePoint`)
    (:`then`
      (`self.K2_SetActorLocationAndRotation` _playercharacter (`self.K2_GetActorLocation` _savepoint) (`self.K2_GetActorRotation` _savepoint) false true)
      (`HealthComponent.SetHealthAlpha` (`/Game/Actors/Characters/Player/PlayerCharacter.HealthComponentPlayer` _playercharacter) 1.0))
    (:`else`)))

(fn `SetSavePoint`
  (params (Point :type "/Game/Actors/Environment/BP_PlayerSavePoint Object Reference"))
  (bind _output_get (set `self.SavePoint` Point))
  (if (not (`/Game/Actors/Environment/BP_PlayerSavePoint.bFirstPoint` _output_get))
    (`KismetSystemLibrary.PrintString` "Set New Save Point")))

(fn `UserConstructionScript`)