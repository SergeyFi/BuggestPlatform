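; BP_PlayerSavePoint is a placeable checkpoint that registers itself with BuggestPlatformGameModeBase_BP as the current save point.
; A point flagged FirstPoint registers on BeginPlay and has its trigger box collision disabled.
; Other points register when player 0's character overlaps the box, then disable and hide it so they fire once.
; The construction script picks the billboard sprite from FirstPoint and sets box visibility from SaveBoxVisible.
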(event `self.ReceiveBeginPlay`
  (if (`self.bFirstPoint`)
    (`self.SavePoint`)))

(event `self.Box.OnComponentBeginOverlap`
  (params (OverlappedComponent :type "PrimitiveComponent Object Reference") (OtherActor :type "Actor Object Reference") (OtherComp :type "PrimitiveComponent Object Reference") (OtherBodyIndex :type Integer) (bFromSweep :type Boolean) (SweepResult :type "HitResult Structure (by ref)"))
  (if (== OtherActor (`GameplayStatics.GetPlayerCharacter` 0))
    (`PrimitiveComponent.SetCollisionEnabled` (`self.Box`) "NoCollision")
    (`self.SavePoint`)
    (`SceneComponent.SetHiddenInGame` (`self.Box`) true false)))

(fn `SavePoint`
  (bind _asbuggest_platform_game_mode_base_bp (cast `/Game/Others/GameModes/BuggestPlatformGameModeBase_BP` (`GameplayStatics.GetGameMode`)))
  (`/Game/Others/GameModes/BuggestPlatformGameModeBase_BP.SetSavePoint` _asbuggest_platform_game_mode_base_bp self))

(fn `UserConstructionScript`
  (bind _box (`self.Box`))
  (bind _bsaveboxvisible (`self.bSaveBoxVisible`))
  (`BillboardComponent.SetSprite` (`self.Billboard`) (select `bool` (`self.bFirstPoint`) :`false` "/Engine/EditorResources/S_NavP.S_NavP" :`true` "/Engine/EditorResources/Spawn_Point.Spawn_Point" :!type "Texture2D Object Reference"))
  (`SceneComponent.SetVisibility` _box _bsaveboxvisible false)
  (`PrimitiveComponent.SetCollisionEnabled` _box (select `bool` (`self.bFirstPoint`) :`false` "QueryOnly" :`true` "NoCollision" :!type "ECollisionEnabled Enum"))
  (`SceneComponent.SetHiddenInGame` _box (not _bsaveboxvisible) false))